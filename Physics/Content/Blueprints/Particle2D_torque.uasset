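; A 2D physics particle actor that rotates under a constant torque, using helper functions defined outside this file.
; On BeginPlay it destroys itself if disabled, otherwise sets mass, center of mass and moment of inertia from its starting location.
; Each Tick integrates rotation with explicit Euler, then applies a constant force at a fixed point and updates angular acceleration.
; The actor transform follows the 2D position at fixed height, with rotation mapped to roll.
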(event EventBeginPlay
  (if (Variables|Default|GetisEnabled)
    (bind _output_get (Variables|Default|Setposition (Math|Conversions|ToVector2D(Vector) (Transformation|GetActorLocation))))
    (Class|Particle2D|SetMass (Variables|Default|Getmass))
    (Variables|Default|SetcenterOfMass _output_get)
    (Class|Particle2D|SetMomentOfInertia)
    (else
      (Actor|DestroyActor))))

(event Collision|EventActorBeginOverlap
  (params (OtherActor :type Actor%20Object%20Reference)))

(event EventTick
  (params (DeltaSeconds :type Float%20%28single-precision%29))
  (Class|Particle2D|UpdateRotationEulerExplicit DeltaSeconds)
  (Class|Particle2D|ApplyTorque (Variables|Default|Getconst_pf) (Variables|Default|Getconst_force))
  (Class|Particle2D|UpdateAngularAcceleration)
  (Transformation|SetActorLocationAndRotation (Math|Conversions|ToVector(Vector2D) (Variables|Default|Getposition) 7e+01) (Math|Rotator|MakeRotator (Variables|Default|Getrotation) 0.0 0.0)))

(fn ConstructionScript)