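; Particle2D_Gravity is a 2D physics particle actor that falls under gravity, simulated in the XZ plane.
; BeginPlay seeds an unset 2D Position from the actor's world location.
; Each Tick kinematically integrates position and rotation, adds a gravity force scaled by mass from inverse mass, then updates acceleration.
; The result is written back to the actor transform with Y fixed at zero and Rotation applied as yaw.
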(event EventBeginPlay
  (bind _returnvalue (Transformation|GetActorLocation))
  (bind (_x _y _z) (Math|Vector|BreakVector _returnvalue))
  (if (Class|KismetMathLibrary|EqualExactlyVector2DVector2D (Variables|Default|Getposition))
    (Variables|Default|Setposition (Math|Vector2D|MakeVector2D _x _z))))

(event Collision|EventActorBeginOverlap
  (params (OtherActor :type Actor%20Object%20Reference)))

(event EventTick
  (params (DeltaSeconds :type Float%20%28single-precision%29))
  (bind _position (Variables|Default|Getposition))
  (bind (_x _y) (Math|Vector2D|BreakVector2D _position))
  ;[1 1 1] Integration
  (Class|Particle2D|UpdatePositionKinematic DeltaSeconds)
  (Class|Particle2D|UpdateRotationKinematic DeltaSeconds)
  (bind _returnvalue (Class|ForceGenerator|GenerateGravity (/ 1.0 (Variables|Default|GetmassInv)) 9.8e+02 "(X=0.000000,Y=-1.000000)"))
  (Class|Particle2D|AddForce _returnvalue)
  (Class|Particle2D|UpdateAcceleration) ; Apply Forces
  ;[1 1 1] Set Position / Rotation
  (Transformation|SetActorLocationAndRotation (Math|Vector|MakeVector _x 0.0 _y) (Math|Rotator|MakeRotator 0.0 0.0 (Variables|Default|Getrotation))))

(fn ConstructionScript)