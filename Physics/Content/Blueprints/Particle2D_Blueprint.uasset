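; Particle2D actor that moves as a simulated 2D particle, driven by a time-varying sideways acceleration.
; Each Tick advances the state with explicit Euler integration, then sets a sine-wave X acceleration that takes effect on the next step.
; It then maps the 2D position to a world location at fixed height and builds the actor's rotation from the particle's two rotation axes.
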(event EventBeginPlay)

(event Collision|EventActorBeginOverlap
  (params (OtherActor :type Actor%20Object%20Reference)))

(event EventTick
  (params (DeltaSeconds :type Float%20%28single-precision%29))
  (bind _rotation (Variables|Default|Getrotation))
  (bind (_x _y) (Math|Vector2D|BreakVector2D _rotation))
  (Class|Particle2D|UpdatePositionsExplicitEuler DeltaSeconds)
  (Variables|Default|Setacceleration (Math|Vector2D|MakeVector2D (* (Math|Trig|Sin(Radians) (Utilities|Time|GetTimeSeconds)) 2e+02) 0.0))
  (Transformation|SetActorLocationAndRotation (Math|Conversions|ToVector(Vector2D) (Variables|Default|Getposition) 5e+01) (Math|Rotator|MakeRotfromXY (Math|Conversions|ToVector(Float) _x) (Math|Conversions|ToVector(Float) _y))))

(fn ConstructionScript)